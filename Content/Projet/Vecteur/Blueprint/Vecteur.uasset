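; Grid manager actor for a tile-based tactical game, handling cube coordinates, character move areas and character moves.
; On BeginPlay it derives each Cube's 2D coordinates from its offset to this actor divided by cube size, then stores cubes in a coordinate dictionary.
; Clicking a cube registers its character with GameManager and spreads a move area through orthogonal neighbours, using decreasing MoveRange.
; OnMovePerso attaches that character to SelectCube, while CheckEnnemiRadius toggles enemy selection.
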(event `CheckEnnemiRadius`
  (params (PersoClick :type "/Game/Projet/Perso/Blueprint/Perso Object Reference"))
  (bind _selectennemi (`self.SelectEnnemi`))
  (if (`KismetArrayLibrary.Array_Contains` _selectennemi PersoClick)
    (`KismetArrayLibrary.Array_RemoveItem` _selectennemi PersoClick)
    (else
      (`KismetArrayLibrary.Array_AddUnique` _selectennemi PersoClick))))

(event `OnMovePerso`
  (bind _selectcube (`self.SelectCube`))
  (bind _returnvalue (`GameplayStatics.GetActorOfClass` "/Game/Projet/GameManager/Blueprint/GameManager.GameManager_C"))
  (bind _selectperso (`/Game/Projet/GameManager/Blueprint/GameManager.SelectPerso` _returnvalue))
  (`self.K2_AttachToActor` _selectperso _selectcube "None" "KeepRelative" "KeepRelative" "KeepRelative" true)
  (`self.K2_SetActorLocation` _selectperso (+ (`self.K2_GetActorLocation` _selectcube) (0.0 0.0 18.0)) false false)
  (bind _returnvalue_2 (`GameplayStatics.GetActorOfClass` "/Game/Projet/GameManager/Blueprint/GameManager.GameManager_C"))
  (set `/Game/Projet/Cube/Blueprint/Cube.Personage` (`/Game/Projet/GameManager/Blueprint/GameManager.SelectPerso` _returnvalue_2) (`self.SelectCube`))
  (set `/Game/Projet/GameManager/Blueprint/GameManager.SelectPerso` (`/Game/Projet/GameManager/Blueprint/GameManager.NULLPerso` _returnvalue_2) _returnvalue_2))

(event `OnClickCube`
  (params (CubeSelect :type "/Game/Projet/Cube/Blueprint/Cube Object Reference"))
  (`self.IntermediateCondition` CubeSelect)
  (`self.ConstructAreaMove`))

(event `self.ReceiveBeginPlay`
  ;[1 1 1] Set information for all the cube about a 2D vector
  ;;[1 1 1] Positionne l'objet dans le cube parent
  (`self.K2_SetActorLocation` (`self.K2_GetActorLocation` (`self.GetAttachParentActor`)))
  ;;[1 1 1] Défini les variables vecteurs dans tous les cubes
  (bind _outactors (`GameplayStatics.GetAllActorsOfClass` "/Game/Projet/Cube/Blueprint/Cube.Cube_C"))
  (`self.SetVectorXY` _outactors)
  ;;[1 1 1] Initialize dictionnary
  (for _array_element _outactors
    (`BlueprintMapLibrary.Map_Add` (`self.CubeDictionnary`) (make `IntVector` (`/Game/Projet/Cube/Blueprint/Cube.VectorX` _array_element) (`/Game/Projet/Cube/Blueprint/Cube.VectorY` _array_element)) _array_element)))

(fn `AnalyseIfPersoInCube`
  (bind _output_get (set `self.SelectCube` null)))

(fn `ConstructAreaMove`
  (bind _outactors (`GameplayStatics.GetAllActorsOfClass` "/Game/Projet/Cube/Blueprint/Cube.Cube_C"))
  (for _array_element _outactors
    (if (not (and (== (`/Game/Projet/Cube/Blueprint/Cube.VectorX` _array_element) (`/Game/Projet/Cube/Blueprint/Cube.VectorX` (`self.SelectCube`))) (== (`/Game/Projet/Cube/Blueprint/Cube.VectorY` _array_element) (`/Game/Projet/Cube/Blueprint/Cube.VectorY` (`self.SelectCube`)))))
      (set `/Game/Projet/Cube/Blueprint/Cube.AllierMoveArea` false _array_element)
      (set `/Game/Projet/Cube/Blueprint/Cube.MoveRange` 0 _array_element)))
  (bind _output_get (set `self.TabCube` (`|MakeArray`)))
  (`KismetArrayLibrary.Array_AddUnique` _output_get (`self.SelectCube`))
  (for _index (range (`/Game/Projet/Cube/Blueprint/Cube.MoveRange` (`self.SelectCube`)))
    (for _array_element_2 (`self.TabCube`)
      (if (== (`/Game/Projet/Cube/Blueprint/Cube.MoveRange` _array_element_2) (- (`/Game/Projet/Cube/Blueprint/Cube.MoveRange` (`self.SelectCube`)) _index))
        (`self.BoucleCheckAdjacent` _outactors _array_element_2 _index)))))

(fn `GetCubeAtGridPosition`
  (params (x :type Integer) (y :type Integer))
  (returns (Cube :type "/Game/Projet/Cube/Blueprint/Cube Object Reference"))
  (return (`BlueprintMapLibrary.Map_Find` (`self.CubeDictionnary`) (make `IntVector` x y))))

(fn `IntermediateCondition`
  (params (SelectCube :type "/Game/Projet/Cube/Blueprint/Cube Object Reference"))
  (bind _output_get (set `self.SelectCube` SelectCube))
  (`/Engine/EditorBlueprintResources/StandardMacros.IsValid` (`/Game/Projet/Cube/Blueprint/Cube.Personage` _output_get)
    (:`Is Valid`
      (bind _personage (`/Game/Projet/Cube/Blueprint/Cube.Personage` _output_get))
      (set `/Game/Projet/Cube/Blueprint/Cube.MoveRange` (`/Game/Projet/Perso/Blueprint/Perso.NumberMove` _personage) _output_get)
      (set `/Game/Projet/Cube/Blueprint/Cube.AllierMoveArea` true _output_get)
      (bind _returnvalue (`GameplayStatics.GetActorOfClass` "/Game/Projet/GameManager/Blueprint/GameManager.GameManager_C"))
      (set `/Game/Projet/GameManager/Blueprint/GameManager.SelectPerso` _personage _returnvalue))))

(fn `ResetAllCube`
  (bind _outactors (`GameplayStatics.GetAllActorsOfClass` "/Game/Projet/Cube/Blueprint/Cube.Cube_C"))
  (for _array_element _outactors
    (set `/Game/Projet/Cube/Blueprint/Cube.EnnemiAttackArea` false _array_element)
    (set `/Game/Projet/Cube/Blueprint/Cube.MoveRange` 0 _array_element)))

(fn `SetVectorXY`
  (params (Array :type "Array of /Game/Projet/Cube/Blueprint/Cube Object Reference"))
  (bind (_returnvalue_x _returnvalue_y) (`KismetMathLibrary.BreakVector` (`self.K2_GetActorLocation`)))
  ;[1 1 1] Boucle qui compare les positions des cubes afin d'y mettre les coordonées de vecteurs 2D
  (for _array_element Array
    (bind (_returnvalue_x_2 _returnvalue_y_2) (`KismetMathLibrary.BreakVector` (`self.K2_GetActorLocation` _array_element)))
    (bind (_returnvalue_x_3 _returnvalue_y_3) (`KismetMathLibrary.BreakVector` (`SceneComponent.K2_GetComponentScale` (`/Game/Projet/Cube/Blueprint/Cube.Cube` _array_element))))
    (bind (_min _max) (`StaticMeshComponent.GetLocalBounds` (`/Game/Projet/Cube/Blueprint/Cube.Cube` _array_element)))
    (set `/Game/Projet/Cube/Blueprint/Cube.VectorX` (`self.CalculVector` _returnvalue_x_2 _returnvalue_x (* (* _returnvalue_x_3 (- (.x _max) (.x _min))) -1.0)) _array_element)
    (set `/Game/Projet/Cube/Blueprint/Cube.VectorY` (`self.CalculVector` _returnvalue_y_2 _returnvalue_y (* _returnvalue_y_3 (- (.y _max) (.y _min)))) _array_element)))

(fn `UserConstructionScript`)